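; BP_Gun is a weapon the player can pick up, drop and fire, starting in the dropped state.
; SetGunState switches mesh physics and collision between Dropped and Equipped, and interaction hands the gun to the player.
; Fire spawns a bullet and muzzle effect at the muzzle socket, aiming the bullet at a far point along the camera's forward vector so shots converge on the view center.
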(event Collision|EventActorBeginOverlap
  (params (OtherActor :type Actor%20Object%20Reference))
  (|CallParentFunction OtherActor) ; This node is disabled and will not be called.\nDrag off pins to build functionality.
)

(event EventTick
  (params (DeltaSeconds :type Float%20%28single-precision%29))
  (|CallParentFunction DeltaSeconds) ; This node is disabled and will not be called.\nDrag off pins to build functionality.
)

(event EventOnInteractedPlayer
  (params (Player :type Ue%204ASP%20Character%20Object%20Reference))
  (Default|PickUpWeapon Player self)
  (Private|SetGunState "NewEnumerator1"))

(event EventBeginPlay
  (Private|SetGunState "NewEnumerator0"))

(fn ConstructionScript
  (|CallParentFunction))

(fn GetInteractionText
  (return "Pick Up"))

(fn InteractionTextAttach
  (return (Variables|Default|GetSkeletalMesh_0)))

(fn SetGunState
  (params (New%20Gun%20State :type EnumGunState%20Enum :default "NewEnumerator0"))
  (bind _skeletalmesh_0 (Variables|Default|GetSkeletalMesh_0))
  (bind _skeletalmesh_0_2 (Variables|Default|GetSkeletalMesh_0))
  (bind _output_get (Variables|Private|SetGun%20State New%20Gun%20State))
  (switch Utilities|FlowControl|Switch|SwitchonEnumGunState _output_get
    (:NewEnumerator0
      (Collision|SetCollisionProfileName (Variables|Default|GetSphere_0) "OverlapAllDynamic" true :!class /Script/Engine.PrimitiveComponent)
      (Physics|SetSimulatePhysics _skeletalmesh_0_2 true)
      (Collision|SetCollisionProfileName _skeletalmesh_0_2 "DropWeapon" true :!class /Script/Engine.PrimitiveComponent))
    (:NewEnumerator1
      (Collision|SetCollisionProfileName (Variables|Default|GetSphere_0) "NoCollision" true :!class /Script/Engine.PrimitiveComponent)
      (Physics|SetSimulatePhysics _skeletalmesh_0 false)
      (Collision|SetCollisionProfileName _skeletalmesh_0 "NoCollision" true :!class /Script/Engine.PrimitiveComponent)
      (Transformation|ResetRelativeTransform _skeletalmesh_0))))

(fn Drop
  (Private|SetGunState "NewEnumerator0"))

(fn Fire
  (params (Player%20Camera :type Camera%20Component%20Object%20Reference))
  (bind _skeletalmesh_0 (Variables|Default|GetSkeletalMesh_0))
  (bind _returnvalue (Transformation|GetSocketLocation _skeletalmesh_0 "b_gun_muzzleflash"))
  (Game|SpawnActorfromClass "/Game/Items/Welpons/BP_Bullet.BP_Bullet_C" (Math|Transform|MakeTransform _returnvalue "0, 0, 0" "1,1,1") "Undefined" 0 (* (Math|Vector|Normalize (- (+ (Transformation|GetWorldLocation Player%20Camera) (* (Math|Vector|GetForwardVector Player%20Camera) 1e+04)) _returnvalue)) 1e+04) 0)
  (Game|SpawnActorfromClass "/Game/Items/Welpons/BP_Muzzel.BP_Muzzel_C" (Math|Transform|MakeTransform _returnvalue "0, 0, 0" "1,1,1") "Undefined" 0 0))